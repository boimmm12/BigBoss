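; BP_Pintu is an interactable door that swings its Hinge between closed and open rotations.
; BeginPlay stores the starting rotation as closed and builds the open rotation by replacing yaw with OpenAngle.
; Interact toggles a Timeline forward or backward, whose Alpha drives a rotator lerp on the Hinge.
; Interacting mid-swing reverses the Timeline from its current position toward closed, leaving IsOpen unchanged.
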(event `self.ReceiveBeginPlay`
  (bind _output_get (set `self.ClosedRot` (`SceneComponent.RelativeRotation` (`self.Hinge`))))
  (set `self.OpenRot` (`KismetMathLibrary.MakeRotator` (.roll _output_get) (.pitch _output_get) (`self.OpenAngle`))))

(event `/Game/TESTIS/Task/BPI_Interact.Interact`
  (params (Actor :type "/Game/ThirdPerson/Blueprints/BP_ThirdPersonCharacter Object Reference"))
  (if (`self.IsOpening`)
    (bind (_direction _alpha) (`Timeline|Timeline` :!via `Reverse` :!label _label)
      (:`Update`
        (`SceneComponent.K2_SetRelativeRotation` (`self.Hinge`) (`KismetMathLibrary.RLerp` (`self.ClosedRot`) (`self.OpenRot`) _alpha) false false))
      (:`Finished`
        (set `self.IsOpening` false)))
    (elif (`self.IsOpen`)
      (set `self.IsOpening` true)
      (set `self.IsOpen` false)
      (goto _label :!via `ReverseFromEnd`)
      (else
        (set `self.IsOpening` true)
        (set `self.IsOpen` true)
        (goto _label :!via `PlayFromStart`)))))

(fn `UserConstructionScript`)