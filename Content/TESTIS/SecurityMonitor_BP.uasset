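; Security monitor actor that shows a live feed from one of its linked security cameras on its screen mesh.
; On BeginPlay, after a short delay, it creates a dynamic screen material and feeds it the first camera's scene capture through a render target.
; SwapCamera cycles through the cameras, creating a new render target sized by viewport and camera quality each time.
; NewPlayerInput forwards horizontal and vertical input to rotate the current camera.
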(event `self.ReceiveBeginPlay`
  (bind (_returnvalue_x _returnvalue_y) (`KismetMathLibrary.BreakVector2D` (`WidgetLayoutLibrary.GetViewportSize`)))
  (bind _cameraqualitylevel (`/Game/TESTIS/SecurityCamera_BP.CameraQualityLevel` (`|GetArrayItem` (`self.LinkedCameras`))))
  (`KismetSystemLibrary.Delay` 0.2)
  (`/Engine/EditorBlueprintResources/StandardMacros.IsValid` (`|GetArrayItem` (`self.LinkedCameras`))
    (:`Is Valid`
      (bind _returnvalue (`KismetMaterialLibrary.CreateDynamicMaterialInstance` "/Game/TESTIS/SecurityCamera_MAT.SecurityCamera_MAT"))
      (bind _output_get (set `self.Camera_MAT` _returnvalue))
      (`PrimitiveComponent.SetMaterial` (`self.Monitor`) 0 _output_get)
      (bind _returnvalue_2 (`KismetRenderingLibrary.CreateRenderTarget2D` (`KismetMathLibrary.FTrunc` (* _returnvalue_x _cameraqualitylevel)) (`KismetMathLibrary.FTrunc` (* _returnvalue_y _cameraqualitylevel))))
      (bind _output_get_2 (set `self.Camera_RT` _returnvalue_2))
      (bind _output_get_3 (set `SceneCaptureComponent2D.TextureTarget` _output_get_2 (`/Game/TESTIS/SecurityCamera_BP.SceneCaptureComponent2D` (`|GetArrayItem` (`self.LinkedCameras`)))))
      (`MaterialInstanceDynamic.SetTextureParameterValue` (`self.Camera_MAT`) "Texture" _output_get_3)
      (`MaterialInstanceDynamic.SetScalarParameterValue` (`self.Camera_MAT`) "Screen Brightness" (`self.Screen Brightness`)))))

(event `SwapCamera`
  (bind (_returnvalue_x _returnvalue_y) (`KismetMathLibrary.BreakVector2D` (`WidgetLayoutLibrary.GetViewportSize`)))
  (bind _currentcamera (`self.CurrentCamera`))
  (bind _cameraqualitylevel (`/Game/TESTIS/SecurityCamera_BP.CameraQualityLevel` (`|GetArrayItem` (`self.LinkedCameras`) (`self.CurrentCamera`))))
  (set `SceneCaptureComponent2D.TextureTarget` null (`/Game/TESTIS/SecurityCamera_BP.SceneCaptureComponent2D` (`|GetArrayItem` (`self.LinkedCameras`) (`self.CurrentCamera`))))
  (`/Engine/EditorBlueprintResources/StandardMacros.IncrementInt` _currentcamera
    (:`  `
      (if (>= _currentcamera (`KismetArrayLibrary.Array_Length` (`self.LinkedCameras`)))
        (set `self.CurrentCamera` 0))
      (bind _returnvalue (`KismetRenderingLibrary.CreateRenderTarget2D` (`KismetMathLibrary.FTrunc` (* _returnvalue_x _cameraqualitylevel)) (`KismetMathLibrary.FTrunc` (* _returnvalue_y _cameraqualitylevel))))
      (bind _output_get (set `self.Camera_RT` _returnvalue))
      (bind _output_get_2 (set `SceneCaptureComponent2D.TextureTarget` _output_get (`/Game/TESTIS/SecurityCamera_BP.SceneCaptureComponent2D` (`|GetArrayItem` (`self.LinkedCameras`) (`self.CurrentCamera`)))))
      (`MaterialInstanceDynamic.SetTextureParameterValue` (`self.Camera_MAT`) "Texture" _output_get_2))))

(event `NewPlayerInput`
  (params (HorizontalValue :type "Float (double-precision)") (VerticalValue :type "Float (double-precision)"))
  (`/Game/TESTIS/SecurityCamera_BP.RotateCamera` (`|GetArrayItem` (`self.LinkedCameras`) (`self.CurrentCamera`)) HorizontalValue VerticalValue))

(fn `UserConstructionScript`)