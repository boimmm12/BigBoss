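; Game manager that runs the workday cycle, shuffling BP_Barang drop targets, picking a drink and showing day start/over widgets.
; Tick, disabled at BeginPlay, advances a scaled clock, flags the noon break and ends the day at 17:00.
; Day end destroys any carried item, increments the GameInstance day, resets or respawns items and re-randomizes.
; DaysVariable defines per-day anomaly difficulty but is not called here; whiteboard Pairing never runs.
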(event `self.ReceiveBeginPlay`
  (bind _returnvalue (`GameplayStatics.GetPlayerController` 0))
  ; BeginPlay
  (`self.RandomizerTargetBarang`)
  (`self.RandomizerDrink`)
  (`WidgetBlueprintLibrary.SetInputMode_UIOnlyEx` _returnvalue null)
  (bind _returnvalue_2 (`|CreateWidget` "/Game/TESTIS/UI/WB_DayStart.WB_DayStart_C"))
  (bind _output_get (set `self.WBDay` _returnvalue_2))
  (`UserWidget.AddToViewport` _output_get 0)
  (set `PlayerController.bShowMouseCursor` true _returnvalue)
  (`self.SetActorTickEnabled` false))

(event `self.ReceiveTick`
  (params (DeltaSeconds :type "Float (single-precision)"))
  (bind _returnvalue (`GameplayStatics.GetPlayerController` 0))
  (bind _allitemspawns (`self.AllItemSpawns`))
  ;[0.05545 0.15 0.07471 0.5] Daily Time
  (if (not (`self.IsDayOver`))
    (bind _output_get (set `self.CurrentTime` (+ (* DeltaSeconds (`self.TimeSpeed`)) (`self.CurrentTime`))))
    (if (and (>= _output_get 12.0) (< _output_get 13.0))
      (set `self.IsBreak` true)
      (else
        (set `self.IsBreak` false)))
    ;[0.09134 0.15 0.1232 0.5] DayIncrement
    (if (>= (`self.CurrentTime`) 17.0)
      (set `self.IsDayOver` true)
      (bind _asbp_third_person_character (cast `/Game/ThirdPerson/Blueprints/BP_ThirdPersonCharacter` (`GameplayStatics.GetPlayerCharacter` 0)))
      (if (`/Game/ThirdPerson/Blueprints/BP_ThirdPersonCharacter.IsCarryingItem` _asbp_third_person_character)
        (for _array_element _allitemspawns
          (bind _carrieditem (`/Game/ThirdPerson/Blueprints/BP_ThirdPersonCharacter.CarriedItem` _asbp_third_person_character))
          (if (== _carrieditem (`.ItemRef_10_FCF252284260C312BEEAD8AD75AAD172` (break `/Game/TESTIS/SaveGame/ItemSpawnData` _array_element)))
            (bind _structout (setmembers `/Game/TESTIS/SaveGame/ItemSpawnData` :`StructRef` _array_element))
            (`KismetArrayLibrary.Array_Set` _allitemspawns 0 (make `/Game/TESTIS/SaveGame/ItemSpawnData` (break `/Game/TESTIS/SaveGame/ItemSpawnData` _structout) (`.InitialTransform_6_B8D8F63C409FE3E60B5BD68906E12FA7` (break `/Game/TESTIS/SaveGame/ItemSpawnData` _structout)) null (`.TargetDrop_15_2ECCAB734725D711251D76B9A5F7E7F8` (break `/Game/TESTIS/SaveGame/ItemSpawnData` _structout))))))
        (`self.K2_DestroyActor` _carrieditem)
        (set `/Game/ThirdPerson/Blueprints/BP_ThirdPersonCharacter.IsCarryingItem` false _asbp_third_person_character))
      (bind _aswb_gi_game (cast `/Game/TESTIS/SaveGame/WB_GI_Game` (`GameplayStatics.GetGameInstance`)))
      (set `/Game/TESTIS/SaveGame/WB_GI_Game.CurrentDay` (+ (`/Game/TESTIS/SaveGame/WB_GI_Game.CurrentDay` _aswb_gi_game) 1) _aswb_gi_game)
      (`self.Respawn`)
      (`self.RandomizerTargetBarang`)
      (`self.RandomizerDrink`)
      ;[0.15 0.04326 0.02165 0.5] Widget Day Over
      (`/Engine/EditorBlueprintResources/StandardMacros.IsValid` (`self.Day Over REF`)
        (:`Is Not Valid`
          (bind _returnvalue_2 (`|CreateWidget` "/Game/TESTIS/UI/WB_DayOver.WB_DayOver_C" (`GameplayStatics.GetPlayerController` 0)))
          (bind _output_get_2 (set `self.Day Over REF` _returnvalue_2))
          (`UserWidget.AddToViewport` _output_get_2 0)
          (`WidgetBlueprintLibrary.SetInputMode_UIOnlyEx` _returnvalue null)
          (set `PlayerController.bShowMouseCursor` true _returnvalue))))))

(event `Respawn`
  (bind _allitemspawns (`self.AllItemSpawns`))
  ; Respawn
  (for _array_element _allitemspawns
    (bind (_itemclass _initialtransform _itemref) (break `/Game/TESTIS/SaveGame/ItemSpawnData` _array_element))
    (`/Engine/EditorBlueprintResources/StandardMacros.IsValid` _itemref
      (:`Is Valid`
        (`/Game/TESTIS/Task/AnterBarang/BP_Barang.ResetLocation` _itemref))
      (:`Is Not Valid`
        (`|SpawnActorFromClass` _itemclass _initialtransform "Undefined" "MultiplyWithRoot" null null)
        (bind _structout (setmembers `/Game/TESTIS/SaveGame/ItemSpawnData` :`StructRef` _array_element))
        (`KismetArrayLibrary.Array_Set` _allitemspawns 0 (make `/Game/TESTIS/SaveGame/ItemSpawnData` (break `/Game/TESTIS/SaveGame/ItemSpawnData` _structout) (`.InitialTransform_6_B8D8F63C409FE3E60B5BD68906E12FA7` (break `/Game/TESTIS/SaveGame/ItemSpawnData` _structout)) (`.ItemRef_10_FCF252284260C312BEEAD8AD75AAD172` (break `/Game/TESTIS/SaveGame/ItemSpawnData` _structout)) (`.TargetDrop_15_2ECCAB734725D711251D76B9A5F7E7F8` (break `/Game/TESTIS/SaveGame/ItemSpawnData` _structout))))))))

(fn `DaysVariable`
  ;[0.15 0.02244 0.1075 0.5] Days Variable
  (switch `int` (`self.CurrentDay`)
    (:`0`
      (set `self.NPCPerAnomali` 1)
      (set `self.AnomaliInterval` (3.3 4.0)) ; Dalam Ment
      (set `self.AnomaliDuration` 0.433) ; Dalam Detik
    )
    (:`1`
      (set `self.NPCPerAnomali` 2)
      (set `self.AnomaliInterval` (3.0 3.3))
      (set `self.AnomaliDuration` 0.4))
    (:`2`
      (set `self.NPCPerAnomali` 2)
      (set `self.AnomaliInterval` (2.3 3.0))
      (set `self.AnomaliDuration` 0.366))
    (:`3`
      (set `self.NPCPerAnomali` 3)
      (set `self.AnomaliInterval` (2.0 2.3))
      (set `self.AnomaliDuration` 0.333))
    (:`4`
      (set `self.NPCPerAnomali` 3)
      (set `self.AnomaliInterval` (1.3 2.0))
      (set `self.AnomaliDuration` 0.3))
    (:`5`
      (set `self.NPCPerAnomali` 4)
      (set `self.AnomaliInterval` (1.0 1.3))
      (set `self.AnomaliDuration` 0.266))
    (:`6`
      (set `self.NPCPerAnomali` 4)
      (set `self.AnomaliInterval` (0.5 1.0))
      (set `self.AnomaliDuration` 0.233))))

(fn `Pairing`
  (locals (ArrBarang :type "Array of /Game/TESTIS/Task/AnterBarang/BP_Barang Object Reference") (ArrPapanTulis :type "Array of /Game/TESTIS/Task/AnterBarang/BP_PapanTulis Object Reference"))
  (bind _outactors (`GameplayStatics.GetAllActorsOfClass` "/Game/TESTIS/Task/AnterBarang/BP_Barang.BP_Barang_C"))
  (set `local.ArrBarang` _outactors)
  (bind _outactors_2 (`GameplayStatics.GetAllActorsOfClass` "/Game/TESTIS/Task/AnterBarang/BP_PapanTulis.BP_PapanTulis_C"))
  (set `local.ArrPapanTulis` _outactors_2)
  (for _array_element (`local.ArrBarang`)
    (for _array_element_2 (`local.ArrPapanTulis`)
      (if (== (`/Game/TESTIS/Task/AnterBarang/BP_PapanTulis.Name` _array_element_2) (`/Game/TESTIS/Task/AnterBarang/BP_Barang.Name` _array_element))
        (set `/Game/TESTIS/Task/AnterBarang/BP_Barang.WhiteboardREF` _array_element_2 _array_element))))
  (`KismetArrayLibrary.Array_Clear` (`local.ArrBarang`))
  (`KismetArrayLibrary.Array_Clear` (`local.ArrPapanTulis`)))

(fn `RandomizerDrink`
  (locals (ArrayTarget :type "Array of Name"))
  (bind _arraytarget (`local.ArrayTarget`))
  (bind _outactors (`GameplayStatics.GetAllActorsOfClass` "/Game/TESTIS/Task/Drink/BP_Drink.BP_Drink_C"))
  (for (_array_element _array_index) _outactors
    (`KismetArrayLibrary.Array_Add` (`local.ArrayTarget`) (`/Game/TESTIS/Task/Drink/BP_Drink.Name` _array_element)))
  (`KismetArrayLibrary.Array_Shuffle` _arraytarget)
  (bind _aswb_gi_game (cast `/Game/TESTIS/SaveGame/WB_GI_Game` (`GameplayStatics.GetGameInstance`)))
  (set `/Game/TESTIS/SaveGame/WB_GI_Game.SelectedDrink` (`|GetArrayItem` _arraytarget _array_index) _aswb_gi_game))

(fn `RandomizerTargetBarang`
  (locals (ArrayTarget :type "Array of Name"))
  (`KismetArrayLibrary.Array_Shuffle` (`local.ArrayTarget`))
  (bind _outactors (`GameplayStatics.GetAllActorsOfClass` "/Game/TESTIS/Task/AnterBarang/BP_Barang.BP_Barang_C"))
  (for (_array_element _array_index) _outactors
    (set `/Game/TESTIS/Task/AnterBarang/BP_Barang.TargetDrop` (`|GetArrayItem` (`local.ArrayTarget`) _array_index) _array_element))
  (`/Game/TESTIS/Task/AnterBarang/BP_Barang.SpawnData` _outactors))

(fn `UserConstructionScript`)