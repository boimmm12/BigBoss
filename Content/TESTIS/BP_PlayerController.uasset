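; Player controller that owns the game's HUD widgets for the day cycle, interaction prompt and CCTV overlay.
; On BeginPlay it creates all six widgets, adds all but the restart widget to the viewport, and shows only the day-start screen.
; Custom events toggle each widget's visibility or block look and move input.
; EndPlay calls the game instance's auto-save message for any end reason.
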(event `self.ReceiveBeginPlay`
  (bind _returnvalue (`|CreateWidget` "/Game/TESTIS/UI/WB_Daily.WB_Daily_C" self))
  (bind _output_get (set `self.WB Daily` _returnvalue))
  (bind _returnvalue_2 (`|CreateWidget` "/Game/TESTIS/UI/WB_DayStart.WB_DayStart_C" self))
  (bind _output_get_2 (set `self.WB Start` _returnvalue_2))
  (bind _returnvalue_3 (`|CreateWidget` "/Game/TESTIS/UI/WB_DayOver.WB_DayOver_C" self))
  (bind _output_get_3 (set `self.WB Over` _returnvalue_3))
  (bind _returnvalue_4 (`|CreateWidget` "/Game/TESTIS/UI/WB_Interact.WB_Interact_C" self))
  (bind _output_get_4 (set `self.WB Interact` _returnvalue_4))
  (bind _returnvalue_5 (`|CreateWidget` "/Game/TESTIS/UI/WB_CCTVOverlayButton.WB_CCTVOverlayButton_C" self))
  (bind _output_get_5 (set `self.WB CCTV Overlay` _returnvalue_5))
  (bind _returnvalue_6 (`|CreateWidget` "/Game/TESTIS/UI/WB_Restart.WB_Restart_C" self))
  (bind _output_get_6 (set `self.WB Restart` _returnvalue_6))
  (`UserWidget.AddToViewport` _output_get 0)
  (`UserWidget.AddToViewport` _output_get_2 0)
  (`UserWidget.AddToViewport` _output_get_3 0)
  (`UserWidget.AddToViewport` _output_get_4 0)
  (`UserWidget.AddToViewport` _output_get_5 0)
  (`Widget.SetVisibility` _output_get "Collapsed")
  (`Widget.SetVisibility` _output_get_3 "Collapsed")
  (`Widget.SetVisibility` _output_get_4 "Collapsed")
  (`Widget.SetVisibility` _output_get_5 "Collapsed")
  (`Widget.SetVisibility` _output_get_6 "Collapsed")
  (`Widget.SetVisibility` _output_get_2 "Visible"))

(event `/Game/TESTIS/UI/BPI_HUD.DailyUI`
  (params (SetVisibile :type Boolean))
  (bind _wb_daily (`self.WB Daily`))
  (`/Engine/EditorBlueprintResources/StandardMacros.IsValid` _wb_daily
    (:`Is Valid`
      (if SetVisibile
        (`Widget.SetVisibility` _wb_daily "Visible")
        (else
          (`Widget.SetVisibility` _wb_daily "Collapsed"))))))

(event `/Game/TESTIS/UI/BPI_HUD.DailyStartUI`
  (params (NewParam :type Boolean))
  (bind _wb_start (`self.WB Start`))
  (`/Engine/EditorBlueprintResources/StandardMacros.IsValid` _wb_start
    (:`Is Valid`
      (if NewParam
        (`Widget.SetVisibility` _wb_start "Visible")
        (else
          (`Widget.SetVisibility` _wb_start "Collapsed"))))))

(event `/Game/TESTIS/UI/BPI_HUD.DailyOverUI`
  (params (NewParam :type Boolean))
  (bind _wb_over (`self.WB Over`))
  (`/Engine/EditorBlueprintResources/StandardMacros.IsValid` _wb_over
    (:`Is Valid`
      (if NewParam
        (`Widget.SetVisibility` _wb_over "Visible")
        (else
          (`Widget.SetVisibility` _wb_over "Collapsed"))))))

(event `/Game/TESTIS/UI/BPI_HUD.InteractUI`
  (params (NewParam :type Boolean))
  (bind _wb_interact (`self.WB Interact`))
  (`/Engine/EditorBlueprintResources/StandardMacros.IsValid` _wb_interact
    (:`Is Valid`
      (if NewParam
        (`Widget.SetVisibility` _wb_interact "Visible")
        (else
          (`Widget.SetVisibility` _wb_interact "Collapsed"))))))

(event `/Game/TESTIS/UI/BPI_HUD.CCTVInteractUI`
  (params (NewParam :type Boolean))
  (bind _wb_cctv_overlay (`self.WB CCTV Overlay`))
  (`/Engine/EditorBlueprintResources/StandardMacros.IsValid` _wb_cctv_overlay
    (:`Is Valid`
      (if NewParam
        (`Widget.SetVisibility` _wb_cctv_overlay "Visible")
        (else
          (`Widget.SetVisibility` _wb_cctv_overlay "Collapsed"))))))

(event `/Game/TESTIS/UI/BPI_HUD.ControllerInput`
  (params (NewParam :type Boolean))
  (`self.SetIgnoreLookInput` NewParam)
  (`self.SetIgnoreMoveInput` NewParam))

(event `/Game/TESTIS/UI/BPI_HUD.DayRestartUI`
  (params (NewParam :type Boolean))
  (bind _wb_restart (`self.WB Restart`))
  (`/Engine/EditorBlueprintResources/StandardMacros.IsValid` _wb_restart
    (:`Is Valid`
      (if NewParam
        (`Widget.SetVisibility` _wb_restart "Visible")
        (else
          (`Widget.SetVisibility` _wb_restart "Collapsed"))))))

(event `self.ReceiveEndPlay`
  (params (EndPlayReason :type "EEndPlayReason Enum" :default "Destroyed"))
  (switch `EEndPlayReason` EndPlayReason
    (:`Destroyed`
      _)
    (:`LevelTransition`
      _)
    (:`EndPlayInEditor`
      _)
    (:`RemovedFromWorld`
      _)
    (:`Quit`
      _))
  (message `/Game/TESTIS/SaveGame/BPI_Save.AutoSave` (`GameplayStatics.GetGameInstance`)))

(fn `UserConstructionScript`)