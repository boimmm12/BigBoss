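; BP_CCTV is a security camera actor that renders its view to a render target and can be aimed.
; On BeginPlay, CCTVID selects which of two render targets (CCTV_CAM_1 or CCTV_CAM_2) the SceneCaptureComponent2D writes to.
; RotateCamera adds sensitivity-scaled horizontal and vertical input to the capture component's relative yaw and pitch, clamped to per-camera rotation limits with roll held at zero.
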(event `self.ReceiveBeginPlay`
  (bind _scenecapturecomponent2d (`self.SceneCaptureComponent2D`))
  (switch `int` (`self.CCTV ID`)
    (:`0`
      (set `SceneCaptureComponent2D.TextureTarget` "/Game/TESTIS/IniYangTest/CCTV_CAM_1.CCTV_CAM_1" _scenecapturecomponent2d))
    (:`1`
      (set `SceneCaptureComponent2D.TextureTarget` "/Game/TESTIS/IniYangTest/CCTV_CAM_2.CCTV_CAM_2" _scenecapturecomponent2d))))

(fn `RotateCamera`
  (params (HorizontalShift :type "Float (double-precision)") (VerticalShift :type "Float (double-precision)"))
  (bind (_relativerotation_roll _relativerotation_pitch _relativerotation_yaw) (`KismetMathLibrary.BreakRotator` (`SceneComponent.RelativeRotation` (`self.SceneCaptureComponent2D`))))
  (`SceneComponent.K2_SetRelativeRotation` (`self.SceneCaptureComponent2D`) (`KismetMathLibrary.MakeRotator` 0.0 (`KismetMathLibrary.FClamp` (+ _relativerotation_pitch (* (`local.VerticalShift`) (`self.VerticalSens`))) (`self.MaxDownRotation`) (`self.MaxUpRotation`)) (`KismetMathLibrary.FClamp` (+ _relativerotation_yaw (* (`local.HorizontalShift`) (`self.HorizontalSens`))) (`self.MaxLeftRotation`) (`self.MaxRightRotation`))) false false))

(fn `UserConstructionScript`)