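; NPC staff Blueprint that picks its current animation from a normal pool or an anomaly pool, based on whether it is flagged as an anomaly.
; NextAnim selects a random entry from the matching pool.
; A looping timer started at BeginPlay re-rolls the normal animation periodically, leaving anomaly staff unchanged.
; Getter functions expose the current animation and anomaly flag.
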(event `/Game/TESTIS/Task/Anomali/BPI_Anim.NextAnim`
  (bind _anomalipool (`self.AnomaliPool`))
  (bind _normalpool (`self.NormalPool`))
  (if (`self.IsAnomali`)
    (set `self.StaffAnim` (`|GetArrayItem` _anomalipool (`KismetMathLibrary.RandomIntegerInRange` 0 (- (`KismetArrayLibrary.Array_Length` _anomalipool) 1))))
    (else
      (set `self.StaffAnim` (`|GetArrayItem` _normalpool (`KismetMathLibrary.RandomIntegerInRange` 0 (- (`KismetArrayLibrary.Array_Length` _normalpool) 1)))))))

(event `self.ReceiveBeginPlay`
  (`parent.ReceiveBeginPlay`)
  (`KismetSystemLibrary.K2_SetTimerDelegate` (delegate `/Game/TESTIS/Task/Anomali/BPI_Anim.IdleAnim`) 5.0 true))

(event `/Game/TESTIS/Task/Anomali/BPI_Anim.IdleAnim`
  (bind _normalpool (`self.NormalPool`))
  (if (not (`self.IsAnomali`))
    (set `self.StaffAnim` (`|GetArrayItem` _normalpool (`KismetMathLibrary.RandomIntegerInRange` 0 (- (`KismetArrayLibrary.Array_Length` _normalpool) 1))))))

(fn `IsAnomaliAnim`
  (returns (IsAnomali :type Boolean))
  (return (`self.IsAnomali`)))

(fn `StaffAnimation`
  (returns (NewParam :type "/Game/TESTIS/Task/Anomali/Staff/E_AnimNPCStaff Enum"))
  (return (`self.StaffAnim`)))

(fn `UserConstructionScript`
  (`parent.UserConstructionScript`))