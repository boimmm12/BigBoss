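; BP_NPCMeeting is a meeting NPC that picks which animation it plays, with normal and anomaly variants.
; NextAnim chooses a random MeetingAnim from AnomaliPool or NormalPool depending on IsAnomali.
; A looping timer started on BeginPlay re-rolls a normal animation periodically, leaving anomalous NPCs unchanged.
; MeetingAnimation and IsAnomaliAnim expose the current animation and anomaly flag to other Blueprints.
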(event `/Game/TESTIS/Task/Anomali/BPI_Anim.NextAnim`
  (bind _normalpool (`self.NormalPool`))
  (bind _anomalipool (`self.AnomaliPool`))
  (if (`self.IsAnomali`)
    (set `self.MeetingAnim` (`|GetArrayItem` _anomalipool (`KismetMathLibrary.RandomIntegerInRange` 0 (- (`KismetArrayLibrary.Array_Length` _anomalipool) 1))))
    (else
      (set `self.MeetingAnim` (`|GetArrayItem` _normalpool (`KismetMathLibrary.RandomIntegerInRange` 0 (- (`KismetArrayLibrary.Array_Length` _normalpool) 1)))))))

(event `self.ReceiveBeginPlay`
  (`parent.ReceiveBeginPlay`)
  (`KismetSystemLibrary.K2_SetTimerDelegate` (delegate `/Game/TESTIS/Task/Anomali/BPI_Anim.IdleAnim`) 5.0 true))

(event `/Game/TESTIS/Task/Anomali/BPI_Anim.IdleAnim`
  (bind _normalpool (`self.NormalPool`))
  (if (not (`self.IsAnomali`))
    (set `self.MeetingAnim` (`|GetArrayItem` _normalpool (`KismetMathLibrary.RandomIntegerInRange` 0 (- (`KismetArrayLibrary.Array_Length` _normalpool) 1))))))

(fn `IsAnomaliAnim`
  (returns (IsAnomali :type Boolean))
  (return (`self.IsAnomali`)))

(fn `MeetingAnimation`
  (returns (MeetingAnim :type "/Game/TESTIS/Task/Anomali/Meeting/E_AnimNPCMeeting Enum"))
  (return (`self.MeetingAnim`)))

(fn `UserConstructionScript`
  (`parent.UserConstructionScript`))