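; BP_Drink is an interactable drink that raises or lowers the player's sanity when consumed.
; On Interact, it compares its Name to the drink message from the GameInstance, adding sanity on a match, subtracting the same amount otherwise, then calling a sanity check.
; A CanDrink flag with a short delay blocks repeated use.
; The BreakTime, Drink and Sanity getters return only default values.
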(event `self.ReceiveBeginPlay`
  ; BeginPlay
  (set `self.ConsumedDrink` self))

(event `/Game/TESTIS/Task/BPI_Interact.Interact`
  (params (Actor :type "/Game/ThirdPerson/Blueprints/BP_ThirdPersonCharacter Object Reference"))
  (bind _returnvalue (`GameplayStatics.GetGameInstance`))
  ; Drink
  (if (`self.CanDrink`)
    (bind _today_sdrink (message `/Game/TESTIS/Task/BPI_Task.Get Drink` (`GameplayStatics.GetGameInstance`)))
    (if (== _today_sdrink (`self.Name`))
      (bind _sanity (message `/Game/TESTIS/Task/BPI_Task.Get Sanity` _returnvalue))
      (message `/Game/TESTIS/Task/BPI_Task.Set Sanity` _returnvalue (+ _sanity 20.0))
      (else
        (bind _sanity_2 (message `/Game/TESTIS/Task/BPI_Task.Get Sanity` _returnvalue))
        (message `/Game/TESTIS/Task/BPI_Task.Set Sanity` _returnvalue (- _sanity_2 20.0))))
    (message `/Game/TESTIS/Task/BPI_Task.CheckSanity` (`GameplayStatics.GetGameInstance`))
    (set `self.CanDrink` false)
    (`KismetSystemLibrary.Delay` 2.0)
    (set `self.CanDrink` true)))

(fn `Get BreakTime`
  (returns (IsBreakCalled :type Boolean))
  (return false))

(fn `Get Drink`
  (returns (`Today'sDrink` :type Name))
  (return "None"))

(fn `Get Sanity`
  (returns (Sanity :type "Float (double-precision)"))
  (return 0.0))

(fn `UserConstructionScript`)