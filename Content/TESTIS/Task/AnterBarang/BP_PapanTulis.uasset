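; Whiteboard actor for the AnterBarang (item delivery) task that displays its drop target as text.
; On BeginPlay it binds to the GameManager game mode's Randomized event, then writes TargetDrop to its TextRender when that fires and unbinds all listeners from the event.
; SetTargetDrop stores a new target and calls OnTargetChanged, while SetTargetItem, GetBarang and GetCarrying are empty stubs.
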(event `self.ReceiveBeginPlay`
  (bind _asgm_game_manager (cast `/Game/TESTIS/GM_GameManager` (`GameplayStatics.GetGameMode`)))
  (add `/Game/TESTIS/GM_GameManager.Randomized` _asgm_game_manager (delegate `SetText`)))

(event `SetText`
  (`TextRenderComponent.K2_SetText` (`self.TextRender`) (`KismetTextLibrary.Conv_NameToText` (`self.TargetDrop`)))
  (clear `/Game/TESTIS/GM_GameManager.Randomized` (stale `self.ReceiveBeginPlay` _asgm_game_manager)))

(fn `GetBarang`
  (returns (`Barang REF` :type "/Game/TESTIS/Task/AnterBarang/BP_Barang Object Reference"))
  (return null))

(fn `GetCarrying`
  (returns (IsCarrying :type Boolean))
  (return false))

(fn `SetTargetDrop`
  (params (NewTarget :type Name))
  (set `self.TargetDrop` NewTarget)
  (`self.OnTargetChanged`))

(fn `SetTargetItem`
  (params (BP_barang :type "/Game/TESTIS/Task/AnterBarang/BP_Barang Object Reference")))

(fn `UserConstructionScript`)