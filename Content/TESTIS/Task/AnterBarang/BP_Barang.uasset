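; BP_Barang is a carriable item for a delivery task, tagged with a drop target.
; On BeginPlay it stores its transform, finds the name-matched BP_PapanTulis whiteboard and registers its spawn data with GM_GameManager.
; Overlap sets it as the character's CarriedItem and, if nothing is carried, enables pickup and the interact UI until overlap ends.
; ResetLocation restores its transform, visibility and collision; UpdateWhiteboard is an empty stub.
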(event `self.ReceiveBeginPlay`
  (set `self.InitialTransform` (`self.GetTransform` self))
  (bind _outactors (`GameplayStatics.GetAllActorsOfClass` "/Game/TESTIS/Task/AnterBarang/BP_PapanTulis.BP_PapanTulis_C"))
  (for _array_element _outactors
    (if (== (`/Game/TESTIS/Task/AnterBarang/BP_PapanTulis.Name` _array_element) (`self.Name`))
      (set `self.WhiteboardREF` _array_element)))
  (`self.SpawnData`))

(event `self.Coliision.OnComponentBeginOverlap`
  (params (OverlappedComponent :type "PrimitiveComponent Object Reference") (OtherActor :type "Actor Object Reference") (OtherComp :type "PrimitiveComponent Object Reference") (OtherBodyIndex :type Integer) (bFromSweep :type Boolean) (SweepResult :type "HitResult Structure (by ref)"))
  (bind _asbp_third_person_character (cast `/Game/ThirdPerson/Blueprints/BP_ThirdPersonCharacter` OtherActor))
  (set `/Game/ThirdPerson/Blueprints/BP_ThirdPersonCharacter.CarriedItem` self _asbp_third_person_character)
  (if (not (`/Game/ThirdPerson/Blueprints/BP_ThirdPersonCharacter.IsCarryingItem` _asbp_third_person_character))
    (set `/Game/ThirdPerson/Blueprints/BP_ThirdPersonCharacter.CanPickUp` true _asbp_third_person_character)
    (`Widget.SetVisibility` (`/Game/ThirdPerson/Blueprints/BP_ThirdPersonCharacter.InteractUI REF` _asbp_third_person_character) "Visible")
    (`KismetSystemLibrary.PrintString` (`KismetStringLibrary.Conv_NameToString` (`self.TargetDrop`)))))

(event `self.ReceiveActorEndOverlap`
  (params (OtherActor :type "Actor Object Reference"))
  (bind _asbp_third_person_character (cast `/Game/ThirdPerson/Blueprints/BP_ThirdPersonCharacter` OtherActor))
  (`Widget.SetVisibility` (`/Game/ThirdPerson/Blueprints/BP_ThirdPersonCharacter.InteractUI REF` _asbp_third_person_character) "Hidden")
  (set `/Game/ThirdPerson/Blueprints/BP_ThirdPersonCharacter.CanPickUp` false _asbp_third_person_character))

(event `ResetLocation`
  (bind _box (`self.BOX`))
  (`self.K2_SetActorTransform` self (`self.InitialTransform`) false false)
  (`SceneComponent.SetVisibility` _box true false)
  (`PrimitiveComponent.SetCollisionEnabled` _box "QueryAndPhysics"))

(event `SpawnData`
  (bind _asgm_game_manager (cast `/Game/TESTIS/GM_GameManager` (`GameplayStatics.GetGameMode`)))
  (`KismetArrayLibrary.Array_Add` (`/Game/TESTIS/GM_GameManager.AllItemSpawns` _asgm_game_manager) (make `/Game/TESTIS/SaveGame/ItemSpawnData` (`GameplayStatics.GetObjectClass` self) (`self.GetTransform` self) self (`self.TargetDrop`))))

(fn `UpdateWhiteboard`
  (`/Engine/EditorBlueprintResources/StandardMacros.IsValid` (`self.WhiteboardREF`)))

(fn `UserConstructionScript`)