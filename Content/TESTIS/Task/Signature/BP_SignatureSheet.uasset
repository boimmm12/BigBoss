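; Interactable signature sheet for a task in which the player stamps a multi-page document.
; Interacting blends to the sheet's clamped, movable camera and shows the cursor; Q/E cycle wrapped pages by toggling visibility and collision.
; Left-click traces place stamp decals attached to the current page, firing an event on each page's first stamp.
; Four stamped pages raise sanity; the game manager's day-over event clears stamps and exits the view.
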(event `InputMovement`
  (params (X :type "Float (double-precision)") (Y :type "Float (double-precision)"))
  (bind _camera (`self.Camera`))
  (bind (_relativelocation_x _relativelocation_y _relativelocation_z) (`KismetMathLibrary.BreakVector` (`SceneComponent.RelativeLocation` _camera)))
  ; Input Movement, movement camera
  (`SceneComponent.K2_AddLocalOffset` (`self.Camera`) (`KismetMathLibrary.MakeVector` (* (`self.SpeedZ`) X) 0.0 (* Y (`self.SpeedX`))) false false)
  (`SceneComponent.K2_SetRelativeLocation` _camera (`KismetMathLibrary.MakeVector` _relativelocation_x (`KismetMathLibrary.FClamp` _relativelocation_y -100.0 100.0) (`KismetMathLibrary.FClamp` _relativelocation_z 70.0 175.0)) false false))

(event `self.ReceiveBeginPlay`
  (bind _pages (`self.Pages`))
  ; Beginplay
  (`self.EnableInput` (`GameplayStatics.GetPlayerController` 0))
  (for _array_element (`SceneComponent.GetChildrenComponents` (`self.PageRoot`) true)
    (bind _asstatic_mesh_component (cast `StaticMeshComponent` _array_element))
    (`KismetArrayLibrary.Array_Add` _pages _asstatic_mesh_component)
    (`SceneComponent.SetHiddenInGame` _array_element true false)
    (`KismetArrayLibrary.Array_Resize` (`self.StampedPages`) (`KismetArrayLibrary.Array_Length` _pages)))
  (`SceneComponent.SetHiddenInGame` (`|GetArrayItem` (`self.Pages`)) false false)
  (set `self.CurrentPage` 0)
  (bind _asgm_game_manager (cast `/Game/TESTIS/GM_GameManager` (`GameplayStatics.GetGameMode`)))
  (add `/Game/TESTIS/GM_GameManager.DayOver` _asgm_game_manager (delegate `Reset`))
  (add `self.StampAdded` self (delegate `CountStamped`)))

(event `CountStamped`
  (bind _returnvalue (`GameplayStatics.GetGameInstance`))
  ; Beginplay
  (set `self.Stamped` 0)
  (for _array_element (`self.StampedPages`)
    (if _array_element
      (set `self.Stamped` (+ (`self.Stamped`) 1))))
  (if (== (`self.Stamped`) 4)
    (bind _sanity (message `/Game/TESTIS/Task/BPI_Task.Get Sanity` _returnvalue))
    (message `/Game/TESTIS/Task/BPI_Task.Set Sanity` _returnvalue (+ _sanity 20.0))))

(event `Reset`
  (bind _returnvalue (`GameplayStatics.GetPlayerController` 0))
  ; Beginplay
  (for _array_element (`self.SpawnedDecals`)
    (`ActorComponent.K2_DestroyComponent` _array_element))
  (`KismetArrayLibrary.Array_Clear` (`self.SpawnedDecals`))
  (`KismetArrayLibrary.Array_Clear` (`self.StampedPages`))
  (`PlayerController.SetViewTargetWithBlend` _returnvalue (`GameplayStatics.GetPlayerCharacter` 0) 0.5 "VTBlend_Linear" 0.0 false)
  (bind _output_get (set `self.SigningSheet` false))
  (message `/Game/TESTIS/Task/Signature/BPI_Signature.SetSigning` self _output_get)
  (set `PlayerController.bShowMouseCursor` false _returnvalue))

(event `/Game/TESTIS/Task/Signature/BPI_Signature.SetSigning`
  (params (IsSigning :type Boolean))
  ; Interface
  (set `self.SigningSheet` IsSigning))

(event `/Game/TESTIS/Task/BPI_Interact.Interact`
  (params (Actor :type "/Game/ThirdPerson/Blueprints/BP_ThirdPersonCharacter Object Reference"))
  (bind _returnvalue (`GameplayStatics.GetPlayerController` 0))
  (bind _returnvalue_2 (`GameplayStatics.GetPlayerController` 0))
  ; Interact
  (if (`self.SigningSheet`)
    (`PlayerController.SetViewTargetWithBlend` _returnvalue (`GameplayStatics.GetPlayerCharacter` 0) 0.5 "VTBlend_Linear" 0.0 false)
    (bind _output_get (set `self.SigningSheet` false))
    (message `/Game/TESTIS/Task/Signature/BPI_Signature.SetSigning` self _output_get)
    (set `PlayerController.bShowMouseCursor` false _returnvalue)
    (else
      (`PlayerController.SetViewTargetWithBlend` _returnvalue_2 self 0.5 "VTBlend_Linear" 0.0 false)
      (bind _output_get_2 (set `self.SigningSheet` true))
      (message `/Game/TESTIS/Task/Signature/BPI_Signature.SetSigning` self _output_get_2)
      (set `PlayerController.bShowMouseCursor` true _returnvalue_2)
      (set `PlayerController.bEnableClickEvents` true (`GameplayStatics.GetPlayerController` 0)))))

(event `Key|LeftMouseButton`
  (params (Key :type "Key Structure"))
  (bind (_bblockinghit _binitialoverlap _time _distance _location _impactpoint _normal _impactnormal _physmat _hitactor) (`GameplayStatics.BreakHitResult` (`PlayerController.GetHitResultUnderCursorByChannel` (`GameplayStatics.GetPlayerController` 0) "TraceTypeQuery1" true)))
  ; Left Click, Stamp
  (:`Pressed`
    (if (== self _hitactor)
      (bind _returnvalue (`GameplayStatics.SpawnDecalAtLocation` "/Game/TESTIS/Task/Signature/OWI.OWI" (10.0 10.0 25.0) _location))
      (`SceneComponent.K2_AttachToComponent` _returnvalue (`|GetArrayItem` (`self.Pages`) (`self.CurrentPage`)) "None" "KeepWorld" "KeepWorld" "KeepWorld" true)
      (`KismetArrayLibrary.Array_AddUnique` (`self.SpawnedDecals`) _returnvalue)
      (if (not (`|GetArrayItem` (`self.StampedPages`) (`self.CurrentPage`)))
        (`KismetArrayLibrary.Array_Set` (`self.StampedPages`) (`self.CurrentPage`) true)
        (`self.StampAdded` self)))))

(event `Key|Q`
  (params (Key :type "Key Structure"))
  (:`Pressed`
    (if (`self.SigningSheet`)
      (`self.GoToPage` (+ (`self.CurrentPage`) 1)))))

(event `Key|E`
  (params (Key :type "Key Structure"))
  (:`Pressed`
    (if (`self.SigningSheet`)
      (`self.GoToPage` (- (`self.CurrentPage`) 1)))))

(fn `GetSheet`
  (returns (SignatureREF :type "/Game/TESTIS/Task/Signature/BP_SignatureSheet Object Reference"))
  (return self))

(fn `GetSigning`
  (returns (IsSigning :type Boolean))
  (return (`self.SigningSheet`)))

(fn `GoToPage`
  (params (NewParam :type Integer))
  (bind _returnvalue (`KismetArrayLibrary.Array_Length` (`self.Pages`)))
  (bind _output (`|GetArrayItem` (`self.Pages`) (`self.CurrentPage`)))
  (bind _output_2 (`|GetArrayItem` (`self.Pages`) (`self.CurrentPage`)))
  (if (> _returnvalue 0)
    (set `self.WrappedIndex` (mod (+ (mod NewParam _returnvalue) _returnvalue) _returnvalue))
    (`SceneComponent.SetHiddenInGame` _output true true)
    (`PrimitiveComponent.SetCollisionEnabled` _output "NoCollision")
    (set `self.CurrentPage` (`self.WrappedIndex`))
    (`SceneComponent.SetHiddenInGame` _output_2 false true)
    (`PrimitiveComponent.SetCollisionEnabled` _output_2 "QueryOnly")
    (`PrimitiveComponent.SetCollisionResponseToChannel` _output_2 "ECC_Visibility" "ECR_Block")))

(fn `UserConstructionScript`)