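; Game manager that runs the workday clock, day progression and per-day anomaly difficulty, exposing state through message getters and setters.
; Tick, disabled at BeginPlay, advances time, flags the midday break, fires a once-daily sleepy-hour call and ends the day at 17:00 with UI.
; Day changes scale anomaly NPC count, interval and duration.
; It also sends a shuffled drink pick and summed NPC stars to the GameInstance, and restarts days with full sanity.
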(event `self.ReceiveBeginPlay`
  (bind _returnvalue (`GameplayStatics.GetPlayerController` 0))
  ; BeginPlay
  (`self.RandomizerDrink`)
  (`WidgetBlueprintLibrary.SetInputMode_UIOnlyEx` _returnvalue null)
  (set `PlayerController.bShowMouseCursor` true _returnvalue)
  (`self.SetActorTickEnabled` false)
  (message `/Game/TESTIS/Task/Anomali/BPI_NPC.CheckTotalStar` self))

(event `/Game/TESTIS/Task/Anomali/BPI_NPC.CheckTotalStar`
  (set `self.TotalStar` 0)
  (bind _outactors (`GameplayStatics.GetAllActorsWithTag` "NPC"))
  (for _array_element _outactors
    (bind _asbp_npc (cast `/Game/TESTIS/Task/Anomali/BP_NPC` _array_element))
    (set `self.TotalStar` (+ (`/Game/TESTIS/Task/Anomali/BP_NPC.Star` _asbp_npc) (`self.TotalStar`))))
  (message `/Game/TESTIS/Task/Anomali/BPI_NPC.SetTotalStar` (`GameplayStatics.GetGameInstance`) (`self.TotalStar`)))

(event `self.ReceiveTick`
  (params (DeltaSeconds :type "Float (single-precision)"))
  (bind _returnvalue (`GameplayStatics.GetPlayerController` 0))
  (bind _returnvalue_2 (`GameplayStatics.GetPlayerController` 0))
  ;[0.05545 0.15 0.07471 0.5] Daily Time
  (if (not (`self.IsDayOver`))
    (bind _output_get (set `self.CurrentTime` (+ (* DeltaSeconds (`self.TimeSpeed`)) (`self.CurrentTime`))))
    (if (and (>= _output_get 12.0) (< _output_get 13.0))
      (set `self.IsBreak` true)
      (else
        (set `self.IsBreak` false)))
    (`|ExecutionSequence`
      (:`then_0`
        (if (> (`self.CurrentTime`) 13.0)
          (`/Engine/EditorBlueprintResources/StandardMacros.DoOnce` false :!label _label
            (:`Completed`
              (`self.SleepyHour` self)))))
      (:`then_1`
        ;[0.09134 0.15 0.1232 0.5] DayIncrement
        (if (>= (`self.CurrentTime`) 17.0)
          (set `self.IsDayOver` true)
          (`self.DayOver` self)
          (bind _output_get_2 (set `self.CurrentTime` 8.0))
          (`|ExecutionSequence`
            (:`then_0`
              (`/Game/TESTIS/BPI_Time.SetTime` _output_get_2)
              (bind _output_get_3 (set `self.CurrentDay` (+ (`self.CurrentDay`) 1)))
              (`/Game/TESTIS/BPI_Time.SetDay` self _output_get_3)
              (`self.RandomizerDrink`)
              ;[0.15 0.04326 0.02165 0.5] Widget Day Over
              (message `/Game/TESTIS/UI/BPI_HUD.DailyOverUI` _returnvalue_2 true)
              (message `/Game/TESTIS/UI/BPI_HUD.DailyUI` _returnvalue_2 false)
              (`WidgetBlueprintLibrary.SetInputMode_UIOnlyEx` _returnvalue null)
              (set `PlayerController.bShowMouseCursor` true _returnvalue))
            (:`then_1`
              (goto _label :!via `Reset`))))))))

(event `/Game/TESTIS/BPI_Time.SetTime`
  (params (Time :type "Float (double-precision)"))
  ; Interface
  (set `self.CurrentTime` Time))

(event `/Game/TESTIS/Task/Anomali/BPI_NPC.RestartDay`
  (bind _returnvalue (`GameplayStatics.GetPlayerController` 0))
  (bind _returnvalue_2 (`GameplayStatics.GetPlayerController` 0))
  (message `/Game/TESTIS/UI/BPI_HUD.DailyOverUI` _returnvalue true)
  (message `/Game/TESTIS/UI/BPI_HUD.DailyUI` _returnvalue false)
  (`WidgetBlueprintLibrary.SetInputMode_UIOnlyEx` _returnvalue_2 null)
  (set `PlayerController.bShowMouseCursor` true _returnvalue_2)
  (bind _output_get (set `self.CurrentTime` 8.0))
  (`/Game/TESTIS/BPI_Time.SetTime` _output_get)
  (`/Game/TESTIS/BPI_Time.SetDay` self (`self.CurrentDay`))
  (message `/Game/TESTIS/Task/BPI_Task.Set Sanity` (`GameplayStatics.GetGameInstance`) 100.0)
  (set `self.IsDayOver` true))

(event `/Game/TESTIS/BPI_Time.SetDay`
  (params (Day :type Integer))
  ; Interface
  (set `self.CurrentDay` Day))

(event `/Game/TESTIS/Task/Anomali/BPI_Anomali.SetAnomaliInterval`
  (params (AnomaliInterval :type "Vector2D Structure"))
  ; Interface
  (set `self.AnomaliInterval` AnomaliInterval))

(event `/Game/TESTIS/Task/Anomali/BPI_Anomali.SetNPCPerAnomali`
  (params (NPCPerAnomali :type Integer))
  ; Interface
  (set `self.NPCPerAnomali` NPCPerAnomali))

(event `/Game/TESTIS/Task/Anomali/BPI_Anomali.SetAnomaliDuration`
  (params (AnomaliDuration :type "Float (double-precision)"))
  ; Interface
  (set `self.AnomaliDuration` AnomaliDuration))

(event `/Game/TESTIS/BPI_Time.OnDaysChanged`
  ; Interface
  ;;[0.15 0.02244 0.1075 0.5] Days Variable
  (switch `int` (`self.CurrentDay`)
    (:`0`
      (set `self.NPCPerAnomali` 1)
      (set `self.AnomaliInterval` (3.3 4.0)) ; Dalam Ment
      (set `self.AnomaliDuration` 0.433) ; Dalam Detik
    )
    (:`1`
      (set `self.NPCPerAnomali` 2)
      (set `self.AnomaliInterval` (3.0 3.3))
      (set `self.AnomaliDuration` 0.4))
    (:`2`
      (set `self.NPCPerAnomali` 2)
      (set `self.AnomaliInterval` (2.3 3.0))
      (set `self.AnomaliDuration` 0.366))
    (:`3`
      (set `self.NPCPerAnomali` 3)
      (set `self.AnomaliInterval` (2.0 2.3))
      (set `self.AnomaliDuration` 0.333))
    (:`4`
      (set `self.NPCPerAnomali` 3)
      (set `self.AnomaliInterval` (1.3 2.0))
      (set `self.AnomaliDuration` 0.3))
    (:`5`
      (set `self.NPCPerAnomali` 4)
      (set `self.AnomaliInterval` (1.0 1.3))
      (set `self.AnomaliDuration` 0.266))
    (:`6`
      (set `self.NPCPerAnomali` 4)
      (set `self.AnomaliInterval` (0.5 1.0))
      (set `self.AnomaliDuration` 0.233))))

(event `/Game/TESTIS/BPI_Time.SetDayOver`
  (params (IsDayOver :type Boolean))
  ; Interface
  (set `self.IsDayOver` IsDayOver))

(event `/Game/TESTIS/BPI_Time.SetBreak`
  (params (IsBreak :type Boolean))
  ; Interface
  (set `self.IsBreak` IsBreak))

(fn `Get BreakTime`
  (returns (IsBreakCalled :type Boolean))
  (return false))

(fn `Get Drink`
  (returns (`Today'sDrink` :type Name))
  (return "None"))

(fn `Get Sanity`
  (returns (Sanity :type "Float (double-precision)"))
  (return 0.0))

(fn `GetAnomaliDuration`
  (returns (AnomaliDuration :type "Float (double-precision)"))
  (return (`self.AnomaliDuration`)))

(fn `GetAnomaliInterval`
  (returns (AnomaliInterval :type "Vector2D Structure"))
  (return (`self.AnomaliInterval`)))

(fn `GetBreak`
  (returns (IsBreak :type Boolean))
  (return (`self.IsBreak`)))

(fn `GetDay`
  (returns (Day :type Integer))
  (return (`self.CurrentDay`)))

(fn `GetDayOver`
  (returns (IsDayOver :type Boolean))
  (return (`self.IsDayOver`)))

(fn `GetIcon`
  (returns (Icon :type "Texture2D Object Reference"))
  (return null))

(fn `GetName`
  (returns (Name :type Text))
  (return ""))

(fn `GetNPCPerAnomali`
  (returns (NPCPerAnomali :type Integer))
  (return (`self.NPCPerAnomali`)))

(fn `GetRandomizerTimer`
  (returns (RandomizerTimer :type "Float (double-precision)"))
  (return 0.0))

(fn `GetStar`
  (returns (NewParam :type Integer))
  (return 0))

(fn `GetTime`
  (returns (Time :type "Float (double-precision)"))
  (return (`self.CurrentTime`)))

(fn `GetTotalStar`
  (returns (NewParam :type Integer))
  (return 0))

(fn `RandomizerDrink`
  (locals (ArrayTarget :type "Array of Name"))
  (bind _arraytarget (`local.ArrayTarget`))
  (bind _outactors (`GameplayStatics.GetAllActorsOfClass` "/Game/TESTIS/Task/Drink/BP_Drink.BP_Drink_C"))
  (for (_array_element _array_index) _outactors
    (`KismetArrayLibrary.Array_Add` (`local.ArrayTarget`) (`/Game/TESTIS/Task/Drink/BP_Drink.Name` _array_element)))
  (`KismetArrayLibrary.Array_Shuffle` _arraytarget)
  (message `/Game/TESTIS/Task/BPI_Task.Set Drink` (`GameplayStatics.GetGameInstance`) (`|GetArrayItem` _arraytarget _array_index)))

(fn `UserConstructionScript`)