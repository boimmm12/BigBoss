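; GM_Time is a game mode that runs the in-game workday clock, flags a midday break, and ends each day.
; BeginPlay briefly shows a day-start widget, then adds the daily widget.
; Tick advances scaled time until the 17:00 cutoff, then increments the day on the game instance and opens a day-over widget with UI-only input.
; DaysVariable maps the current day to anomaly settings that escalate across seven days.
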(event `self.ReceiveBeginPlay`
  ; BeginPlay
  (`WidgetBlueprintLibrary.SetInputMode_GameOnly` (`GameplayStatics.GetPlayerController` 0))
  (bind _returnvalue (`|CreateWidget` "/Game/TESTIS/UI/WB_DayStart.WB_DayStart_C"))
  (bind _output_get (set `self.WBDay` _returnvalue))
  (`UserWidget.AddToViewport` _output_get 0)
  (`KismetSystemLibrary.Delay` 1.0)
  (`Widget.SetVisibility` (`self.WBDay`) "Hidden")
  (bind _returnvalue_2 (`|CreateWidget` "/Game/TESTIS/UI/WB_Daily.WB_Daily_C"))
  (`UserWidget.AddToViewport` _returnvalue_2 0))

(event `self.ReceiveTick`
  (params (DeltaSeconds :type "Float (single-precision)"))
  (bind _returnvalue (`GameplayStatics.GetPlayerController` 0))
  ;[0.05545 0.15 0.07471 0.5] Daily Time
  (if (not (`self.IsDayOver`))
    (bind _output_get (set `self.CurrentTime` (+ (* DeltaSeconds (`self.TimeSpeed`)) (`self.CurrentTime`))))
    (if (and (>= _output_get 12.0) (< _output_get 13.0))
      (set `self.IsBreak` true)
      (else
        (set `self.IsBreak` false)))
    ;[0.09134 0.15 0.1232 0.5] DayIncrement
    (if (>= (`self.CurrentTime`) 17.0)
      (set `self.IsDayOver` true)
      (bind _aswb_gi_game (cast `/Game/TESTIS/SaveGame/WB_GI_Game` (`GameplayStatics.GetGameInstance`)))
      (set `/Game/TESTIS/SaveGame/WB_GI_Game.CurrentDay` (+ (`/Game/TESTIS/SaveGame/WB_GI_Game.CurrentDay` _aswb_gi_game) 1) _aswb_gi_game)
      ;[0.15 0.04326 0.02165 0.5] Widget Day Over
      (`/Engine/EditorBlueprintResources/StandardMacros.IsValid` (`self.Day Over REF`)
        (:`Is Not Valid`
          (bind _returnvalue_2 (`|CreateWidget` "/Game/TESTIS/UI/WB_DayOver.WB_DayOver_C" (`GameplayStatics.GetPlayerController` 0)))
          (bind _output_get_2 (set `self.Day Over REF` _returnvalue_2))
          (`UserWidget.AddToViewport` _output_get_2 0)
          (`WidgetBlueprintLibrary.SetInputMode_UIOnlyEx` _returnvalue null)
          (set `PlayerController.bShowMouseCursor` true _returnvalue))))))

(fn `DaysVariable`
  ;[0.15 0.02244 0.1075 0.5] Days Variable
  (switch `int` (`self.CurrentDay`)
    (:`0`
      (set `self.NPCPerAnomali` 1)
      (set `self.AnomaliInterval` (3.3 4.0)) ; Dalam Ment
      (set `self.AnomaliDuration` 0.433) ; Dalam Detik
    )
    (:`1`
      (set `self.NPCPerAnomali` 2)
      (set `self.AnomaliInterval` (3.0 3.3))
      (set `self.AnomaliDuration` 0.4))
    (:`2`
      (set `self.NPCPerAnomali` 2)
      (set `self.AnomaliInterval` (2.3 3.0))
      (set `self.AnomaliDuration` 0.366))
    (:`3`
      (set `self.NPCPerAnomali` 3)
      (set `self.AnomaliInterval` (2.0 2.3))
      (set `self.AnomaliDuration` 0.333))
    (:`4`
      (set `self.NPCPerAnomali` 3)
      (set `self.AnomaliInterval` (1.3 2.0))
      (set `self.AnomaliDuration` 0.3))
    (:`5`
      (set `self.NPCPerAnomali` 4)
      (set `self.AnomaliInterval` (1.0 1.3))
      (set `self.AnomaliDuration` 0.266))
    (:`6`
      (set `self.NPCPerAnomali` 4)
      (set `self.AnomaliInterval` (0.5 1.0))
      (set `self.AnomaliDuration` 0.233))))

(fn `UserConstructionScript`)